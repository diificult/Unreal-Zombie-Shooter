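; AI_Character is an enemy that either roams or chases the player and is destroyed when overlapped by an actor tagged Bullet.
; BeginPlay and Tick both set the Bullet tag and switch on the Chase state.
; Roam moves to random navigable points within a radius and Chase moves to the player, each re-calling itself after a short delay on success.
; Explosion effect and sound nodes are present but unconnected.
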(event Custom|Roam
  (AI|AIMoveTo self (.RandomLocation (Class|NavigationSystemV1|GetRandomPointinNavigableRadius (Transformation|GetActorLocation) 5e+02 0 0)) 0 5.0 false
    (:OnSuccess
      (Utilities|FlowControl|Delay 0.5)
      (CallFunction|Roam))))

(event Custom|Chase
  (AI|AIMoveTo self "0, 0, 0" (Game|GetPlayerCharacter 0) 5.0 false
    (:OnSuccess
      (Utilities|FlowControl|Delay 0.5)
      (CallFunction|Chase))))

(event EventBeginPlay
  (Variables|Default|SetBullet "Bullet")
  (switch Utilities|FlowControl|Switch|SwitchonEAIState "NewEnumerator2"
    (:NewEnumerator1
      (CallFunction|Roam))
    (:NewEnumerator2
      (CallFunction|Chase))))

(event Collision|EventActorBeginOverlap
  (params (OtherActor :type Actor%20Object%20Reference))
  (if (Actor|ActorHasTag OtherActor (Variables|Default|GetBullet))
    (Actor|DestroyActor)))

(event EventTick
  (params (DeltaSeconds :type Float%20%28single-precision%29))
  (Variables|Default|SetBullet "Bullet")
  (switch Utilities|FlowControl|Switch|SwitchonEAIState "NewEnumerator2"
    (:NewEnumerator1
      (CallFunction|Roam))
    (:NewEnumerator2
      (CallFunction|Chase))))

(fn ConstructionScript)